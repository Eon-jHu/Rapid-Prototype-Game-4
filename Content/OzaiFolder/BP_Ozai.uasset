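; BP_Ozai is a fire monster that chases the player by retracing their exact path.
; Tick records the first-person character's transform into a queue every frame.
; After a ten-second head start, a looping fixed-interval timer teleports Ozai to the oldest entry and removes it, so the lag varies with frame rate.
; Capsule overlap with the player calls DeathOzaiMessage on the game instance.
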(event `self.ReceiveBeginPlay`
  (`SkeletalMeshComponent.PlayAnimation` (`self.FireMonster`) "/Game/Assets/FireMonster/SK_FireElement_Idle.SK_FireElement_Idle" true)
  (`KismetSystemLibrary.Delay` 10.0)
  (`KismetSystemLibrary.K2_SetTimerDelegate` (delegate `TickTokc`) 0.03 true))

(event `TickTokc`
  (bind _newlocation (`self.NewLocation`))
  (bind (_output_location _output_rotation) (`KismetMathLibrary.BreakTransform` (`|GetArrayItem` _newlocation)))
  (`self.K2_TeleportTo` _output_location _output_rotation)
  (`KismetArrayLibrary.Array_Remove` _newlocation))

(event `self.ReceiveTick`
  (params (DeltaSeconds :type "Float (single-precision)"))
  (bind _asbp_first_person_character (cast `/Game/FirstPerson/Blueprints/BP_FirstPersonCharacter` (`GameplayStatics.GetPlayerCharacter` 0)))
  (`KismetArrayLibrary.Array_Add` (`self.NewLocation`) (`self.GetTransform` _asbp_first_person_character)))

(event `self.Capsule.OnComponentBeginOverlap`
  (params (OverlappedComponent :type "PrimitiveComponent Object Reference") (OtherActor :type "Actor Object Reference") (OtherComp :type "PrimitiveComponent Object Reference") (OtherBodyIndex :type Integer) (bFromSweep :type Boolean) (SweepResult :type "HitResult Structure (by ref)"))
  (cast `/Game/FirstPerson/Blueprints/BP_FirstPersonCharacter` OtherActor)
  (message `/Game/GameManager/BP_InstanceInterface.Death_Ozai` (`GameplayStatics.GetGameInstance`)))

(fn `UserConstructionScript`)