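; BP_bendableBig is a large breakable rock that shatters when a projectile overlaps it and increments the first-person character's IEarth counter.
; The mine event, gated by CanBreak, plays a rockfall sound, swaps the Rock component for a Geometry Collection, and destroys the actor after a delay.
; The overlap handler then clears CanBreak and disables collision on Rock and Box to block repeat hits.
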(event `mine`
  (bind _rock (`self.rock`))
  (if (`self.bCanBreak`)
    (`GameplayStatics.PlaySoundAtLocation` "/Game/toby_playing/Sounds/Rock_Falling_Sound_Effects_All_Sounds__7_.Rock_Falling_Sound_Effects_All_Sounds__7_" (`SceneComponent.RelativeLocation` (`self.rock`)) (struct) 1.0 1.0 0.0 null null null null)
    (`AddComponent|NODE_AddGeometryCollectionComponent-0` :`RelativeTransform` (`KismetMathLibrary.MakeTransform` (`SceneComponent.RelativeLocation` _rock) (`SceneComponent.RelativeRotation` _rock)))
    (`SceneComponent.SetVisibility` (`self.rock`) false false)
    (`ActorComponent.K2_DestroyComponent` (`self.rock`))
    (`KismetSystemLibrary.Delay` 5.0)
    (`self.K2_DestroyActor`)))

(event `self.ReceiveActorBeginOverlap`
  (params (OtherActor :type "Actor Object Reference"))
  (cast `/Game/CollisionContent/BP_ProjectileBase` OtherActor
    (:`then`
      (`self.mine`)
      (set `self.bCanBreak` false)
      (`PrimitiveComponent.SetCollisionEnabled` (`self.rock`) "NoCollision")
      (`PrimitiveComponent.SetCollisionEnabled` (`self.Box`) "NoCollision")
      (bind _asbp_first_person_character (cast `/Game/FirstPerson/Blueprints/BP_FirstPersonCharacter` (`GameplayStatics.GetPlayerPawn` 0)))
      (`/Engine/EditorBlueprintResources/StandardMacros.IncrementInt` (`/Game/FirstPerson/Blueprints/BP_FirstPersonCharacter.iEarth` _asbp_first_person_character)))
    (:`CastFailed`
      (`KismetSystemLibrary.PrintString` "Big bendable cast to projectile failed"))))

(event `self.ReceiveTick`
  (params (DeltaSeconds :type "Float (single-precision)")))

(fn `UserConstructionScript`)