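; BP_WorldRock is a mineable rock that shatters when a projectile hits it and awards the player earth.
; A Box overlap with a BP_ProjectileBase triggers a one-time mine event, gated by CanMine, which increments IEarth on the first-person character and plays a falling-rock sound.
; It swaps the static mesh for a Geometry Collection at the same transform, then destroys the actor after a short delay.
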(event `self.Box.OnComponentBeginOverlap`
  (params (OverlappedComponent :type "PrimitiveComponent Object Reference") (OtherActor :type "Actor Object Reference") (OtherComp :type "PrimitiveComponent Object Reference") (OtherBodyIndex :type Integer) (bFromSweep :type Boolean) (SweepResult :type "HitResult Structure (by ref)"))
  (cast `/Game/CollisionContent/BP_ProjectileBase` OtherActor)
  (`self.mine`))

(event `mine`
  (bind _mesh (`self.Mesh`))
  (if (`self.bCanMine`)
    (set `self.bCanMine` false)
    (`self.IncPlayerEarth`)
    (`GameplayStatics.PlaySoundAtLocation` "/Game/toby_playing/Sounds/Rock_Falling_Sound_Effects_All_Sounds__7_.Rock_Falling_Sound_Effects_All_Sounds__7_" (`SceneComponent.K2_GetComponentLocation` (`self.Mesh`)) (struct) 1.0 1.0 0.0 null null null null)
    (`AddComponent|NODE_AddGeometryCollectionComponent-1` :`RelativeTransform` (`KismetMathLibrary.MakeTransform` (`SceneComponent.RelativeLocation` _mesh) (`SceneComponent.RelativeRotation` _mesh) (`SceneComponent.RelativeScale3D` _mesh)))
    (`SceneComponent.SetVisibility` (`self.Mesh`) false false)
    (`ActorComponent.K2_DestroyComponent` (`self.Mesh`))
    (`KismetSystemLibrary.Delay` 5.0)
    (`self.K2_DestroyActor`)))

(event `IncPlayerEarth`
  (bind _asbp_first_person_character (cast `/Game/FirstPerson/Blueprints/BP_FirstPersonCharacter` (`GameplayStatics.GetPlayerPawn` 0)))
  (`/Engine/EditorBlueprintResources/StandardMacros.IncrementInt` (`/Game/FirstPerson/Blueprints/BP_FirstPersonCharacter.iEarth` _asbp_first_person_character)))

(fn `UserConstructionScript`)