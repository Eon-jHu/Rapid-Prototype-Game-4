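; BP_MeleeWeaponBase is a base Blueprint for melee weapons that performs a hit check when fired or activated.
; After calling the parent logic, it sphere-traces on the Visibility channel from just ahead of the player's first-person camera along its forward vector for MeleeRange, with debug drawing enabled.
; The trace result goes to ApplyOnHit, which is empty here, so this class applies no hit effect itself.
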(event `self.OnFireOrActivate`
  (params (PlayerCharacter :type "/Game/FirstPerson/Blueprints/BP_FirstPersonCharacter Object Reference"))
  (bind _firstpersoncamera (`/Game/FirstPerson/Blueprints/BP_FirstPersonCharacter.FirstPersonCamera` PlayerCharacter))
  (bind _returnvalue (`SceneComponent.GetForwardVector` _firstpersoncamera))
  (bind _returnvalue_2 (`SceneComponent.K2_GetComponentLocation` _firstpersoncamera))
  (`parent.OnFireOrActivate` PlayerCharacter)
  (bind (_outhit _returnvalue_3) (`KismetSystemLibrary.SphereTraceSingle` :`Start` (+ _returnvalue_2 (* _returnvalue 100.0)) :`End` (+ _returnvalue_2 (* _returnvalue (+ 100.0 (`self.MeleeRange`)))) :`Radius` 100.0 :`TraceChannel` "TraceTypeQuery1" :`DrawDebugType` "ForDuration"))
  (`self.ApplyOnHit` _outhit _returnvalue_3))

(fn `ApplyOnHit`
  (params (HitStruct :type "HitResult Structure") (HitAnything :type Boolean)))

(fn `UserConstructionScript`
  (`parent.UserConstructionScript`))