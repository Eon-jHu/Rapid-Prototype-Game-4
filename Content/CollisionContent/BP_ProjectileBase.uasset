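; Base projectile actor that provides contact and release events for launched objects.
; OnProjectileContact spawns an FS_MasterField actor at the given transform and plays the impact sound at the hit location.
; OnProjectileRelease plays a release sound at the static mesh's location, with both sounds skipped if unset.
; The Hit event is deprecated and empty, leaving its old physics impulse and self-destroy logic disconnected, and nothing here calls either custom event.
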(event `self.ReceiveHit`
  (params (MyComp :type "PrimitiveComponent Object Reference") (Other :type "Actor Object Reference") (OtherComp :type "PrimitiveComponent Object Reference") (bSelfMoved :type Boolean) (HitLocation :type "Vector Structure") (HitNormal :type "Vector Structure") (NormalImpulse :type "Vector Structure") (Hit :type "HitResult Structure (by ref)"))
  ;[0.7969 0 0] DEPRECATED Add physics impulse to any physics object we hit
)

(event `OnProjectileContact`
  (params (SpawnTransform :type "Transform Structure") (HitLocation :type "Vector Structure"))
  (`|SpawnActorFromClass` "/Engine/EditorResources/FieldNodes/FS_MasterField.FS_MasterField_C" SpawnTransform "Undefined" "MultiplyWithRoot" null null)
  (bind _impactsound (`self.ImpactSound`)
    (:`then`
      (`GameplayStatics.PlaySoundAtLocation` _impactsound HitLocation (struct) 1.0 1.0 0.0 null null null null))
    (:`else`)))

(event `OnProjectileRelease`
  (bind _projectilereleasesound (`self.ProjectileReleaseSound`)
    (:`then`
      (`GameplayStatics.PlaySoundAtLocation` _projectilereleasesound (`SceneComponent.K2_GetComponentLocation` (`self.StaticMesh`)) (struct) 1.0 1.0 0.0 null null null null))
    (:`else`)))

(fn `UserConstructionScript`)