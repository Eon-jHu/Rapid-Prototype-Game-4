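; BP_Prompt is a spinning trigger actor that shows an on-screen prompt when the first-person character touches it.
; Its capsule overlap creates a new UI_Prompts widget each time, passes the Promptz enum as a string to PromptShow, then adds it to the viewport.
; Tick rotates the root by a fixed step each frame, so spin speed depends on frame rate.
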(event `self.ReceiveTick`
  (params (DeltaSeconds :type "Float (single-precision)"))
  (`SceneComponent.K2_AddRelativeRotation` (`self.DefaultSceneRoot`) (struct :`Yaw` 5.0) false false))

(event `self.Capsule.OnComponentBeginOverlap`
  (params (OverlappedComponent :type "PrimitiveComponent Object Reference") (OtherActor :type "Actor Object Reference") (OtherComp :type "PrimitiveComponent Object Reference") (OtherBodyIndex :type Integer) (bFromSweep :type Boolean) (SweepResult :type "HitResult Structure (by ref)"))
  (cast `/Game/FirstPerson/Blueprints/BP_FirstPersonCharacter` OtherActor)
  (bind _returnvalue (`|CreateWidget` "/Game/UI_Sound/UI_Prompts.UI_Prompts_C"))
  (bind _output_get (set `self.Prompts` _returnvalue))
  (`/Game/UI_Sound/UI_Prompts.PromptShow` _returnvalue (`|GetEnumeratorNameAsString` (`self.Promptz`)))
  (`/Game/UI_Sound/UI_Prompts.PromptShow` _output_get (`|GetEnumeratorNameAsString` (`self.Promptz`)))
  (`UserWidget.AddToViewport` (`self.Prompts`) 0))

(fn `UserConstructionScript`)